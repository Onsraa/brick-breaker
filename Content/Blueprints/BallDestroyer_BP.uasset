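; BallDestroyer_BP is a trigger volume that destroys balls entering it and costs the player a life.
; On BeginPlay it caches the player's Paddle_BP pawn and all Lives_BP actors.
; When a Ball_BP overlaps its Box component, it destroys the ball, decrements the paddle's Lives count and calls UpdateLives on the cached Lives actors.
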(event `self.ReceiveBeginPlay`
  (bind _aspaddle_bp (cast `/Game/Blueprints/Paddle_BP` (`GameplayStatics.GetPlayerPawn` 0)))
  (set `self.As Paddle BP` _aspaddle_bp)
  (bind _outactors (`GameplayStatics.GetAllActorsOfClass` "/Game/Blueprints/Lives_BP.Lives_BP_C"))
  (set `self.Lives Actors` _outactors))

(event `self.Box.OnComponentBeginOverlap`
  (params (OverlappedComponent :type "PrimitiveComponent Object Reference") (OtherActor :type "Actor Object Reference") (OtherComp :type "PrimitiveComponent Object Reference") (OtherBodyIndex :type Integer) (bFromSweep :type Boolean) (SweepResult :type "HitResult Structure (by ref)"))
  (bind _as_paddle_bp (`self.As Paddle BP`))
  (bind _asball_bp (cast `/Game/Blueprints/Ball_BP` OtherActor))
  (`self.K2_DestroyActor` _asball_bp)
  (set `/Game/Blueprints/Paddle_BP.Lives` (- (`/Game/Blueprints/Paddle_BP.Lives` _as_paddle_bp) 1) _as_paddle_bp)
  (`/Game/Blueprints/Lives_BP.UpdateLives` (`self.Lives Actors`)))

(fn `UserConstructionScript`)