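; Lives HUD Blueprint that shows the player paddle's remaining lives as heart sprites.
; On BeginPlay it casts the player pawn to Paddle_BP and caches the reference.
; UpdateLives switches on the paddle's Lives count and swaps one of three sprite components to a different heart sprite for values two, one and zero.
; It only changes sprites on loss, with no path to restore them.
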(event `self.ReceiveBeginPlay`
  (bind _aspaddle_bp (cast `/Game/Blueprints/Paddle_BP` (`GameplayStatics.GetPlayerPawn` 0)))
  (set `self.As Paddle BP` _aspaddle_bp))

(event `self.ReceiveTick`
  (params (DeltaSeconds :type "Float (single-precision)")))

(fn `UpdateLives`
  (switch `int` (`/Game/Blueprints/Paddle_BP.Lives` (`self.As Paddle BP`))
    (:`0`
      (`PaperSpriteComponent.SetSprite` (`self.LivesSprite2`) "/Game/Assets/Lives/Hearts_Sprite_0.Hearts_Sprite_0"))
    (:`1`
      (`PaperSpriteComponent.SetSprite` (`self.LivesSprite1`) "/Game/Assets/Lives/Hearts_Sprite_0.Hearts_Sprite_0"))
    (:`2`
      (`PaperSpriteComponent.SetSprite` (`self.LivesSprite`) "/Game/Assets/Lives/Hearts_Sprite_0.Hearts_Sprite_0"))))

(fn `UserConstructionScript`)