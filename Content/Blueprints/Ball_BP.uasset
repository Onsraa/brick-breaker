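; Ball actor for a paddle game that launches itself and handles the loss of a life.
; On BeginPlay it moves just in front of the player's Paddle_BP and receives a physics impulse at a random angle, scaled by MaxSpeed.
; When destroyed, it asks the spawner for a new ball if Lives exceeds one, otherwise shows the GameOver widget.
; The speed clamp is disconnected, and the two start-position helper functions are not called here.
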(event `self.ReceiveBeginPlay`
  (bind _maxspeed (`self.MaxSpeed`))
  (bind _returnvalue (`KismetMathLibrary.DegreesToRadians` (`KismetMathLibrary.RandomFloatInRange` 40.0 120.0)))
  (bind (_returnvalue_x _returnvalue_y _returnvalue_z) (`KismetMathLibrary.BreakVector` (`SceneComponent.K2_GetComponentLocation` (`Actor.RootComponent` (`self.As Paddle BP`)))))
  (bind _aspaddle_bp (cast `/Game/Blueprints/Paddle_BP` (`GameplayStatics.GetPlayerPawn` 0)))
  (set `self.As Paddle BP` _aspaddle_bp)
  (set `self.StartPosition` (`KismetMathLibrary.MakeVector` (+ _returnvalue_x 25.0) _returnvalue_y _returnvalue_z))
  (`self.SetToStart`)
  (`PrimitiveComponent.AddImpulse` (`self.Ball`) (`KismetMathLibrary.MakeVector` (* (`KismetMathLibrary.Sin` _returnvalue) _maxspeed) (* (`KismetMathLibrary.Cos` _returnvalue) _maxspeed)) "None" false))

(event `self.ReceiveHit`
  (params (MyComp :type "PrimitiveComponent Object Reference") (Other :type "Actor Object Reference") (OtherComp :type "PrimitiveComponent Object Reference") (bSelfMoved :type Boolean) (HitLocation :type "Vector Structure") (HitNormal :type "Vector Structure") (NormalImpulse :type "Vector Structure") (Hit :type "HitResult Structure (by ref)"))
  (bind _returnvalue (`PrimitiveComponent.GetPhysicsLinearVelocity` (`self.Ball`) "None")))

(event `SetToStart`
  (`SceneComponent.K2_SetWorldLocation` (`self.Ball`) (`self.StartPosition`) false false))

(event `self.ReceiveDestroyed`
  (if (> (`/Game/Blueprints/Paddle_BP.Lives` (`self.As Paddle BP`)) 1)
    (`/Game/Blueprints/BallSpawner_BP.SpawnBall` (`self.BallSpawnerRef`))
    (else
      (bind _returnvalue (`|GenericCreateObject` "/Game/Blueprints/GameOver_WB.GameOver_WB_C"))
      (`UserWidget.AddToViewport` _returnvalue 0))))

(fn `FireFromStartPosition`
  (`PrimitiveComponent.AddAngularImpulseInDegrees` (`self.Ball`) (0.0 0.0 0.0) "None" true))

(fn `SetBallToStartPosition`
  (bind (_returnvalue_x _returnvalue_y _returnvalue_z) (`KismetMathLibrary.BreakVector` (`SceneComponent.K2_GetComponentLocation` (`Actor.RootComponent` (`self.As Paddle BP`)))))
  (`SceneComponent.K2_SetWorldLocation` (`self.Ball`) (`KismetMathLibrary.MakeVector` (+ _returnvalue_x 20.0) _returnvalue_y _returnvalue_z) false false))

(fn `UserConstructionScript`)