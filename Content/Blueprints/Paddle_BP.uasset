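; Player paddle Blueprint for a brick breaker game, moved along its X axis by player input.
; BeginPlay adds the Enhanced Input mapping context and creates the player HUD widget.
; Move input applies swept, delta-time-scaled offsets to the paddle component, while Dash applies a one-off swept impulse offset without physics.
; Hits on the paddle component play a 2D sound.
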(event `self.ReceiveBeginPlay`
  (bind _asplayer_controller (cast `PlayerController` (`self.GetController`)))
  (bind _returnvalue (pcsubsystem `EnhancedInputLocalPlayerSubsystem` _asplayer_controller))
  (`/Engine/EditorBlueprintResources/StandardMacros.IsValid` _returnvalue
    (:`Is Valid`
      (`EnhancedInputSubsystemInterface.AddMappingContext` _returnvalue "/Game/Inputs/BrickBreaker_IMC.BrickBreaker_IMC" 0 (struct))
      (bind _returnvalue_2 (`|GenericCreateObject` "/Game/Blueprints/PlayerHUD_WB.PlayerHUD_WB_C"))
      (bind _output_get (set `self.PlayerHud` _returnvalue_2))
      (`UserWidget.AddToViewport` _output_get 0))))

(event `EnhancedInput|/Game/Inputs/Dash_IA`
  (params (ActionValue :type Boolean) (ElapsedSeconds :type "Float (double-precision)") (TriggeredSeconds :type "Float (double-precision)") (InputAction :type "InputAction Object Reference" :default "/Game/Inputs/Dash_IA.Dash_IA"))
  (:`Started`
    (`SceneComponent.K2_AddLocalOffset` (`self.Paddle`) (`KismetMathLibrary.MakeVector` (* (stale `EnhancedInput|/Game/Inputs/Move_IA` ActionValue) (`self.ImpulseForce`))) true false)))

(event `EnhancedInput|/Game/Inputs/Move_IA`
  (params (ActionValue :type "Float (double-precision)") (ElapsedSeconds :type "Float (double-precision)") (TriggeredSeconds :type "Float (double-precision)") (InputAction :type "InputAction Object Reference" :default "/Game/Inputs/Move_IA.Move_IA"))
  (:`Triggered`
    (`SceneComponent.K2_AddLocalOffset` (`self.Paddle`) (`KismetMathLibrary.MakeVector` (* ActionValue (`self.Speed`) (`GameplayStatics.GetWorldDeltaSeconds`))) true false)))

(event `self.Paddle.OnComponentHit`
  (params (HitComponent :type "PrimitiveComponent Object Reference") (OtherActor :type "Actor Object Reference") (OtherComp :type "PrimitiveComponent Object Reference") (NormalImpulse :type "Vector Structure") (Hit :type "HitResult Structure (by ref)"))
  (`GameplayStatics.PlaySound2D` "/Game/Assets/Sounds/Hit_Paddle_Sound.Hit_Paddle_Sound" 1.0 1.0 0.0 null null))

(fn `UserConstructionScript`)