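; Destructible brick for a Breakout-style game, given a random color on BeginPlay and showing more damage as it loses lives.
; Each hit spawns VFX, sound and camera shake, then swaps the damage sprite with a brief flash material.
; At zero lives it destroys itself, updates the paddle HUD's score, and shows the win widget and pauses when no bricks remain.
; ShowImpact and hit-stop helpers exist but are not called here.
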(event `self.ReceiveBeginPlay`
  (bind _bricksprite (`self.BrickSprite`))
  (set `self.InitialMaterial` (`PrimitiveComponent.GetMaterial` (`self.BrickSprite`) 0))
  (bind _aspaddle_bp (cast `/Game/Blueprints/Paddle_BP` (`GameplayStatics.GetPlayerPawn` 0)))
  (set `self.As Paddle BP` _aspaddle_bp)
  (bind _output_get (set `self.Color` (`KismetMathLibrary.RandomInteger` 4)))
  (switch `int` _output_get
    (:`0`
      (`PaperSpriteComponent.SetSprite` _bricksprite "/Game/Assets/Bricks/bricks_Sprite_10.bricks_Sprite_10"))
    (:`1`
      (`PaperSpriteComponent.SetSprite` _bricksprite "/Game/Assets/Bricks/bricks_Sprite_17.bricks_Sprite_17"))
    (:`2`
      (`PaperSpriteComponent.SetSprite` _bricksprite "/Game/Assets/Bricks/bricks_Sprite_24.bricks_Sprite_24"))
    (:`3`
      (`PaperSpriteComponent.SetSprite` _bricksprite "/Game/Assets/Bricks/bricks_Sprite_31.bricks_Sprite_31"))))

(event `self.Brick.OnComponentHit`
  (params (HitComponent :type "PrimitiveComponent Object Reference") (OtherActor :type "Actor Object Reference") (OtherComp :type "PrimitiveComponent Object Reference") (NormalImpulse :type "Vector Structure") (Hit :type "HitResult Structure (by ref)"))
  (bind _bricksprite (`self.BrickSprite`))
  (bind _bricksprite_2 (`self.BrickSprite`))
  (`NiagaraFunctionLibrary.SpawnSystemAtLocation` "/Game/Assets/VFX/Explosion_VFX.Explosion_VFX" (`SceneComponent.K2_GetComponentLocation` (`self.Brick`)))
  (`GameplayStatics.PlaySound2D` "/Game/Assets/Sounds/Hit_Brick_Sound.Hit_Brick_Sound" 1.0 1.0 0.0 null null)
  (bind _asplayer_controller (cast `PlayerController` (`Pawn.GetController` (`self.As Paddle BP`))))
  (`PlayerController.ClientStartCameraShake` :`self` _asplayer_controller :`Shake` "/Game/Blueprints/CameraShake_BP.CameraShake_BP_C")
  (set `self.Lives` (- (`self.Lives`) (`self.DamageTaken`)))
  (switch `int` (`self.Lives`)
    (:`0`
      (`self.K2_DestroyActor`)
      (`/Game/Blueprints/PlayerHUD_WB.Update score` (`/Game/Blueprints/Paddle_BP.PlayerHud` (`self.As Paddle BP`)))
      (bind _outactors (`GameplayStatics.GetAllActorsOfClass` "Brick_BP_C"))
      (if (== (`KismetArrayLibrary.Array_Length` _outactors) 0)
        (bind _returnvalue (`|CreateWidget` "/Game/Blueprints/Win_WP.Win_WP_C"))
        (`UserWidget.AddToViewport` _returnvalue 0)
        (`GameplayStatics.SetGamePaused` true)))
    (:`1`
      (switch `int` (`self.Color`)
        (:`0`
          (`PaperSpriteComponent.SetSprite` _bricksprite "/Game/Assets/Bricks/bricks_Sprite_12.bricks_Sprite_12"))
        (:`1`
          (`PaperSpriteComponent.SetSprite` _bricksprite "/Game/Assets/Bricks/bricks_Sprite_19.bricks_Sprite_19"))
        (:`2`
          (`PaperSpriteComponent.SetSprite` _bricksprite "/Game/Assets/Bricks/bricks_Sprite_26.bricks_Sprite_26"))
        (:`3`
          (`PaperSpriteComponent.SetSprite` _bricksprite "/Game/Assets/Bricks/bricks_Sprite_33.bricks_Sprite_33")))
      (`PrimitiveComponent.SetMaterial` _bricksprite_2 0 "/Game/Materials/DamageFlash_MAT.DamageFlash_MAT" :!label _label)
      (`KismetSystemLibrary.Delay` 0.08)
      (`PrimitiveComponent.SetMaterial` _bricksprite_2 0 (`self.InitialMaterial`)))
    (:`2`
      (switch `int` (`self.Color`)
        (:`0`
          (`PaperSpriteComponent.SetSprite` _bricksprite "/Game/Assets/Bricks/bricks_Sprite_11.bricks_Sprite_11")
          (goto _label))
        (:`1`
          (`PaperSpriteComponent.SetSprite` _bricksprite "/Game/Assets/Bricks/bricks_Sprite_18.bricks_Sprite_18")
          (goto _label))
        (:`2`
          (`PaperSpriteComponent.SetSprite` _bricksprite "/Game/Assets/Bricks/bricks_Sprite_25.bricks_Sprite_25")
          (goto _label))
        (:`3`
          (`PaperSpriteComponent.SetSprite` _bricksprite "/Game/Assets/Bricks/bricks_Sprite_32.bricks_Sprite_32")
          (goto _label))))))

(fn `EndHitStop`
  (set `self.CustomTimeDilation` 1.0))

(fn `ShowImpact`
  (bind _bricksprite (`self.BrickSprite`))
  (`PrimitiveComponent.SetMaterial` _bricksprite 0 "/Game/Materials/DamageFlash_MAT.DamageFlash_MAT")
  (`PrimitiveComponent.SetMaterial` _bricksprite 0 (`self.InitialMaterial`)))

(fn `StartHitStop`
  (params (Duration :type "Float (double-precision)"))
  (set `self.CustomTimeDilation` 0.0)
  (`KismetSystemLibrary.K2_SetTimer` null "EndHitStop" Duration))

(fn `UserConstructionScript`)